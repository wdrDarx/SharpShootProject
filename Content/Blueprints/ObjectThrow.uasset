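; Obstacle thrower actor that, while Activated, spawns randomly sized Obstacle actors around its Spawn point and pushes them along an Axis.
; Two self-repeating Delay loops run from BeginPlay, one spawning at a configurable interval and one moving, both polling Activated.
; New obstacles join an array and trigger ForceNetUpdate.
; The move loop sweeps each valid one through its InterpToMovement component with random Y jitter.
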(event `self.ReceiveBeginPlay`
  (bind _activated_ (`self.activated?`))
  (`|ExecutionSequence`
    (:`then_0`
      (if _activated_ :!label _label
        (`self.spawn obstacle`)
        (`KismetSystemLibrary.Delay` (`self.delay`))
        (goto _label)
        (else
          (`KismetSystemLibrary.Delay` 0.2)
          (goto _label))))
    (:`then_1`
      (if _activated_ :!label _label_2
        (`self.move obstacles`)
        (`KismetSystemLibrary.Delay` 0.02)
        (goto _label_2)
        (else
          (`KismetSystemLibrary.Delay` 0.2)
          (goto _label_2))))))

(event `spawn obstacle`
  (`|ExecutionSequence`
    (:`then_0`
      (bind _returnvalue (`|SpawnActorFromClass` "/Game/Blueprints/Obstacle.Obstacle_C" (`KismetMathLibrary.MakeTransform` (+ (`SceneComponent.K2_GetComponentLocation` (`self.Spawn`)) (`KismetMathLibrary.MakeVector` (`KismetMathLibrary.RandomFloatInRange` -100.0 100.0) (`KismetMathLibrary.RandomFloatInRange` -100.0 200.0) (`KismetMathLibrary.RandomFloatInRange` -100.0 100.0))) (`KismetMathLibrary.RandomRotator` false)) "Undefined" "OverrideRootScale" null "/Game/Levels/Materials/BaseGlow.BaseGlow" (`KismetMathLibrary.MakeVector` (`KismetMathLibrary.RandomFloatInRange` 0.2 1.5) (`KismetMathLibrary.RandomFloatInRange` 0.2 1.5) (`KismetMathLibrary.RandomFloatInRange` 0.2 1.5)) false null))
      (`KismetArrayLibrary.Array_Add` (`self.Obstacles`) _returnvalue)
      (`self.ForceNetUpdate`))))

(event `move obstacles`
  (`self.moveObstacles M`))

(event `moveObstacles M`
  (for _array_element (`self.Obstacles`)
    (`/Engine/EditorBlueprintResources/StandardMacros.IsValid` _array_element
      (:`Is Valid`
        (`MovementComponent.K2_MoveUpdatedComponent` :`self` (`/Game/Blueprints/Obstacle.InterpToMovement` _array_element) :`Delta` (+ (0.0 0.0 0.0) (`self.axis`) (`KismetMathLibrary.MakeVector` 0.0 (`KismetMathLibrary.RandomFloatInRange` -10.0 10.0))))))))

(event `self.ReceiveTick`
  (params (DeltaSeconds :type "Float (single-precision)")))

(fn `UserConstructionScript`)