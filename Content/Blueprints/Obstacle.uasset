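; Obstacle is a Blueprint actor with a Cube mesh that serves as a configurable, optionally rotating obstacle.
; On BeginPlay, a ScaleServer event applies the configured Material and world Scale to the cube, wrapped in ForceNetUpdate calls.
; If Rotate is set, a delayed loop repeatedly nudges the cube's relative rotation toward a new random rotator with a single RInterpTo step per interval.
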(event `scale server`
  (bind _cube (`self.Cube`))
  (`self.ForceNetUpdate`)
  (`PrimitiveComponent.SetMaterial` _cube 0 (`self.Material`))
  (`SceneComponent.SetWorldScale3D` _cube (`self.scale`))
  (`self.ForceNetUpdate`))

(event `self.ReceiveTick`
  (params (DeltaSeconds :type "Float (single-precision)")))

(event `self.ReceiveBeginPlay`
  (bind _cube (`self.Cube`))
  (`|ExecutionSequence`
    (:`then_0`
      (`self.scale server`))
    (:`then_1`
      (if (`self.rotate?`) :!label _label
        (`SceneComponent.K2_SetRelativeRotation` _cube (`KismetMathLibrary.RInterpTo` (`SceneComponent.RelativeRotation` _cube) (`KismetMathLibrary.RandomRotator` false) (`GameplayStatics.GetWorldDeltaSeconds`) 5.0) false false)
        (`KismetSystemLibrary.Delay` (`self.SecondsPerRotaion`))
        (goto _label)))))

(fn `UserConstructionScript`)